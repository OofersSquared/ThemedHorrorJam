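; AC_DialogueTest is a test dialogue component scripting a branching conversation with an NPC named Mom about chores.
; Dialogue switches on DialogueTreeIndex, nesting AddDialogue calls whose Passthrough state and chosen option pick the next line.
; Finishing the chores advances the index to a tree with one random line; other endings rewind or clear dialogue progress before closing the conversation.
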(event EventBeginPlay)

(event EventTick
  (params (DeltaSeconds :type Float%20%28single-precision%29)))

(fn Dialogue
  (|CallParentFunction)
  (switch int (Variables|Default|GetDialogueTreeIndex)
    (:Default
      (bind (_state _option_index) (CallFunction|AddDialogue "Mom" "Hello my son, come help me with my chores. Do your chores!" (Utilities|Array|MakeArray "Yes" "No") :!label _label))
      (switch Utilities|FlowControl|Switch|SwitchonEnum_DialogueState _state
        (:NewEnumerator0
          (switch int _option_index
            (:0
              (bind (_state_2 _option_index_2) (CallFunction|AddDialogue "Mom" "Good job son :)" (Utilities|Array|MakeArray "I have done them." "I have not done them.")))
              (switch Utilities|FlowControl|Switch|SwitchonEnum_DialogueState _state_2
                (:NewEnumerator0
                  (switch int _option_index_2
                    (:0
                      (bind _state_3 (CallFunction|AddDialogue "Mom" "Thank you son." (Utilities|Array|MakeArray "...")))
                      (switch Utilities|FlowControl|Switch|SwitchonEnum_DialogueState _state_3
                        (:NewEnumerator0
                          (CallFunction|SetDialogueTreeIndex 1)
                          (CallFunction|CloseConversation))))
                    (:1
                      (bind _state_4 (CallFunction|AddDialogue "Mom" "Screw you son." (Utilities|Array|MakeArray "...")))
                      (switch Utilities|FlowControl|Switch|SwitchonEnum_DialogueState _state_4
                        (:NewEnumerator0
                          (CallFunction|RemoveDialogueProgress 2)
                          (CallFunction|CloseConversation))))))))
            (:1
              (bind _state_5 (CallFunction|AddDialogue "Mom" "Then drown in your ideals and die." (Utilities|Array|MakeArray "...")))
              (switch Utilities|FlowControl|Switch|SwitchonEnum_DialogueState _state_5
                (:NewEnumerator0
                  (CallFunction|ClearDialogueProgress)
                  (CallFunction|CloseConversation))))))))
    (:0
      (goto _label))
    (:1
      (bind _state_6 (CallFunction|AddDialogue "Mom" (Utilities|Select :Index (Math|Random|RandomIntegerinRange 0 3) :Option%200 "Love you son." :Option%201 "I am an alien" :Option%202 "I'm going to bed." :Option%203 "Go back to your dad son.") (Utilities|Array|MakeArray "...")))
      (switch Utilities|FlowControl|Switch|SwitchonEnum_DialogueState _state_6
        (:NewEnumerator0
          (CallFunction|ClearDialogueProgress)
          (CallFunction|CloseConversation))))))