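; Base dialogue component that opens a W_Dialogue widget with UI-only input and notifies its owner when the conversation closes.
; The empty Dialogue function, apparently a child override, scripts conversations through AddDialogue calls.
; Each choice is saved to a progress map and replays Dialogue from the start: answered steps return stored options, unanswered ones update the widget.
; Progress can be rolled back, cleared or reset by switching dialogue trees.
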(fn OpenConversation
  (bind _returnvalue (UserInterface|CreateWidget "/Game/UI/W_Dialogue.W_Dialogue_C" 0 self))
  (bind _output_get (Variables|Default|SetDialogueWidget _returnvalue))
  (UserInterface|Viewport|AddtoViewport _output_get 0)
  (Input|SetInputModeUIOnly (Game|GetPlayerController 0) 0 "DoNotLock" false)
  (Variables|/Script/Engine.PlayerController|SetbShowMouseCursor (Game|GetPlayerController 0) true)
  (CallFunction|ProgressDialogue))

(fn CloseConversation
  (Widget|RemovefromParent (Variables|Default|GetDialogueWidget))
  (Class|BPIInteractible|ConversationClosed(Message) (Components|GetOwner)))

(fn ProgressDialogue
  (Variables|Default|SetDialogueIndex -1)
  (CallFunction|Dialogue))

(fn Dialogue)

(fn AddDialogue
  (params (NPC%20Name :type Text) (Dialogue :type Text) (Options :type Array%20of%20Texts))
  (bind _dialogueprogress (Variables|Default|GetDialogueProgress))
  (bind _dialogueindex (Variables|Default|GetDialogueIndex))
  (bind (_value _returnvalue) (Utilities|Map|Find _dialogueprogress _dialogueindex))
  (Math|Integer|IncrementInt (Variables|Default|GetDialogueIndex)
    (:%20%20
      (if _returnvalue
        (return "NewEnumerator0" _value)
        (else
          (Default|UpdateDialogueText (Variables|Default|GetDialogueWidget) (Variables|Default|GetDialogueIndex) NPC%20Name Dialogue Options)
          (return "NewEnumerator1" 0))))))

(fn UpdateSelectedOption
  (params (Progress%20Index :type Integer) (Option%20Index :type Integer))
  (Utilities|Map|Add (Variables|Default|GetDialogueProgress) Progress%20Index Option%20Index)
  (CallFunction|ProgressDialogue))

(fn ClearDialogueProgress
  (Utilities|Map|Clear (Variables|Default|GetDialogueProgress)))

(fn RemoveDialogueProgress
  (params (ProgressSteps :type Integer))
  (for _index (range 0 ProgressSteps)
    (Utilities|Map|Remove (Variables|Default|GetDialogueProgress) (- (Variables|Default|GetDialogueIndex) _index))))

(fn SetDialogueTreeIndex
  (params (DialogueTreeIndex :type Integer))
  (Variables|Default|SetDialogueTreeIndex DialogueTreeIndex)
  (CallFunction|ClearDialogueProgress))