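; BP_Mom is an interactable NPC, shown as a sprite, that opens a conversation with the player.
; Each tick it yaws toward the player camera as a billboard, and its construction script fills the name text from CharacterName.
; In interact range it shows the name and applies an outline material; the out-of-range branch only hides the name.
; Interact stores the instigator and opens ACDialogueTest's conversation, then ConversationClosed notifies that instigator.
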(event EventShowInteractible
  (params (canShowInteract? :type Boolean))
  ;[1 1 1] Outlines and shows name when in Interact range
  (if canShowInteract?
    (Rendering|SetVisibility (Variables|Default|GetTXT_CharacterName) true false)
    (Rendering|Material|SetMaterial (Variables|Default|GetKomaeda_Sprite1) 0 "/Game/Assets/Oofers/Materials/InteractibleOutline.InteractibleOutline")
    (else
      (Rendering|SetVisibility (Variables|Default|GetTXT_CharacterName) false false))))

(event EventInteract
  (params (Instigator :type Actor%20Object%20Reference))
  (Variables|Default|SetInteractInstigator Instigator)
  (Default|OpenConversation (Variables|Default|GetAC_DialogueTest)))

(event EventTick
  (params (DeltaSeconds :type Float%20%28single-precision%29))
  ;[1 1 1] Always facing the PlayerCharacter
  (Transformation|SetActorRotation (Math|Rotator|MakeRotator 0.0 0.0 (.Yaw (Math|Rotator|BreakRotator (Math|Rotator|FindLookatRotation (Transformation|GetActorLocation) (Transformation|GetActorLocation (Game|GetPlayerCameraManager 0))))))))

(event EventConversationClosed
  (Class|BPIInteractible|ConversationClosed(Message) (Variables|Default|GetInteractInstigator)))

(fn ConstructionScript
  (Rendering|Components|TextRender|SetText (Variables|Default|GetTXT_CharacterName) (Variables|Default|GetCharacterName)))