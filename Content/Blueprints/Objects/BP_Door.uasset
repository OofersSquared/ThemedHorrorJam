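; BP_Door is an interactable door that swings open or closed each time it receives Interact.
; A timeline plays forward or in reverse to lerp the door mesh's relative rotation, with IsAnimating blocking input until IsOpen flips on finish.
; During each update, door collision is disabled while opening and set to query-only while closing, with debug prints of that state.
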(event EventInteract
  (params (Instigator :type Actor%20Object%20Reference))
  (Variables|Default|SetInteractInstigator Instigator)
  (if (not (Variables|Default|GetisAnimating))
    (Variables|Default|SetisAnimating true)
    (if (Variables|Default|GetisOpen)
      (bind _doorrotation (Timeline|Timeline Reverse)
        (:Update
          (Transformation|SetRelativeRotation (Variables|Default|GetDoor) (Math|Rotator|Lerp(Rotator) "0, 0, 0" "0.000000,-90.000000,0.000000" _doorrotation) false false)
          (if (Variables|Default|GetisOpen)
            (Collision|SetCollisionEnabled (Variables|Default|GetDoorCollision) "QueryOnly")
            (Development|PrintString "enabled")
            (else
              (Collision|SetCollisionEnabled (Variables|Default|GetDoorCollision) "NoCollision")
              (Development|PrintString "disabled"))))
        (:Finished
          (Variables|Default|SetisOpen (not (Variables|Default|GetisOpen)))
          (Variables|Default|SetisAnimating false)))
      (else
        (Timeline|Timeline PlayFromStart)))))

(fn ConstructionScript)