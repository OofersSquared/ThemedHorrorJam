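; Player character Blueprint handling Enhanced Input movement, camera look and interaction with nearby objects.
; BeginPlay adds the default mapping context; move follows control rotation and look scales pitch by a sensitivity value.
; An InteractRadius overlap tracks one BPI_Interactible at a time, toggling its prompt, and the interact action messages it.
; A ConversationClosed event hides the cursor and restores game-only input.
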(event OnComponentBeginOverlap(InteractRadius)
  (params (OverlappedComponent :type Primitive%20Component%20Object%20Reference) (OtherActor :type Actor%20Object%20Reference) (OtherComp :type Primitive%20Component%20Object%20Reference) (OtherBodyIndex :type Integer) (bFromSweep :type Boolean) (SweepResult :type Hit%20Result%20Structure%20%28by%20ref%29))
  (if (!= OtherActor self)
    (if (Utilities|DoesObjectImplementInterface OtherActor "/Game/Blueprints/BPI_Interactible.BPI_Interactible_C")
      (Utilities|IsValid (Variables|Default|GetInteractible)
        (:Is%20Valid
          (Class|BPIInteractible|ShowInteractible(Message) (Variables|Default|GetInteractible) false)
          (Variables|Default|SetInteractible 0))
        (:Is%20Not%20Valid
          _))
      (Variables|Default|SetInteractible OtherActor)
      (Class|BPIInteractible|ShowInteractible(Message) (Variables|Default|GetInteractible) true))))

(event OnComponentEndOverlap(InteractRadius)
  (params (OverlappedComponent :type Primitive%20Component%20Object%20Reference) (OtherActor :type Actor%20Object%20Reference) (OtherComp :type Primitive%20Component%20Object%20Reference) (OtherBodyIndex :type Integer))
  (if (and (!= OtherActor self) (== (Variables|Default|GetInteractible) OtherActor))
    (Class|BPIInteractible|ShowInteractible(Message) (Variables|Default|GetInteractible) false)
    (Variables|Default|SetInteractible 0)))

(event Input|EnhancedActionEvents|EnhancedInputActionIA_Interact
  (params (ActionValue :type Boolean) (ElapsedSeconds :type Float%20%28double-precision%29) (TriggeredSeconds :type Float%20%28double-precision%29) (InputAction :type Input%20Action%20Object%20Reference :default "/Game/Input/Actions/IA_Interact.IA_Interact"))
  (:Triggered
    (Utilities|IsValid (Variables|Default|GetInteractible)
      (:Is%20Valid
        (Class|BPIInteractible|Interact(Message) (Variables|Default|GetInteractible) self)))))

(event Input|EnhancedActionEvents|EnhancedInputActionIA_Move
  (params (ActionValue :type Vector%202D%20Structure) (ElapsedSeconds :type Float%20%28double-precision%29) (TriggeredSeconds :type Float%20%28double-precision%29) (InputAction :type Input%20Action%20Object%20Reference :default "/Game/Input/Actions/IA_Move.IA_Move"))
  ;[1 1 1] Moement Controls
  ;;[1 1 1] Left/Right Movement
  (Pawn|Input|AddMovementInput (Math|Vector|GetRightVector (Pawn|GetControlRotation :!class /Script/Engine.Pawn)) (.x ActionValue) false)
  ;;[1 1 1] Forward/Backward Movement
  (Pawn|Input|AddMovementInput (Math|Vector|GetForwardVector (Pawn|GetControlRotation :!class /Script/Engine.Pawn)) (.y ActionValue) false))

(event Input|EnhancedActionEvents|EnhancedInputActionIA_Look
  (params (ActionValue :type Vector%202D%20Structure) (ElapsedSeconds :type Float%20%28double-precision%29) (TriggeredSeconds :type Float%20%28double-precision%29) (InputAction :type Input%20Action%20Object%20Reference :default "/Game/Input/Actions/IA_Look.IA_Look"))
  ;[1 1 1] Camera Controls
  (Pawn|Input|AddControllerYawInput (.x ActionValue))
  (Pawn|Input|AddControllerPitchInput (* (.y ActionValue) (Variables|Default|GetPitchSensitivity))))

(event EventBeginPlay
  ;[1 1 1] Add Input System
  (bind _asplayer_controller (Utilities|Casting|CastToPlayerController (Pawn|GetController)))
  (Utilities|IsValid (PlayerController|LocalPlayerSubsystems|GetEnhancedInputLocalPlayerSubsystem _asplayer_controller)
    (:Is%20Valid
      (Input|AddMappingContext (PlayerController|LocalPlayerSubsystems|GetEnhancedInputLocalPlayerSubsystem _asplayer_controller) "/Game/Input/IMC_default.IMC_default" 0 "(bIgnoreAllPressedKeysUntilRelease=True,bForceImmediately=False,bNotifyUserSettings=False)"))))

(event EventConversationClosed
  (bind _returnvalue (Game|GetPlayerController 0))
  (Variables|/Script/Engine.PlayerController|SetbShowMouseCursor _returnvalue false)
  (Input|SetInputModeGameOnly _returnvalue false))

(fn ConstructionScript)